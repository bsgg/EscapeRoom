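; Lobby player controller that relays movement and inventory navigation input for the player's character.
; It caches the pawn as MainCharacter on BeginPlay and forwards move axes to it.
; Left and right actions print debug text and call ClientNavigateInventory directly, bypassing the active-inventory check in OnInventoryNavigate.
; Logic for interacting, selecting items, toggling the inventory with input locking, and ending navigation is disconnected and never runs.
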(event EventBeginPlay
  ;[1 1 1] Set Character
  (bind _asmain_character (Utilities|Casting|CastToMainCharacter (Pawn|GetControlledPawn)))
  (Variables|Default|SetMyCharacter _asmain_character))

(event Input|ActionEvents|InputActionInteract
  (params (Key :type Key%20Structure)))

(event Input|ActionEvents|InputActionNavigateInventoryLeft
  (params (Key :type Key%20Structure))
  (:Pressed
    ;[1 1 1] Inventory Navigation
    (Development|PrintString "NavigateLeft")
    (Class|LobbyPlayerController|ClientNavigateInventory "VE_LEFT")))

(event Input|ActionEvents|InputActionNavigateInventoryRight
  (params (Key :type Key%20Structure))
  (:Pressed
    ;[1 1 1] Inventory Navigation
    (Development|PrintString "NavigateRight")
    (Class|LobbyPlayerController|ClientNavigateInventory "VE_RIGHT")))

(event Input|AxisEvents|InputAxisMoveForward
  (params (AxisValue :type Float%20%28single-precision%29))
  (bind _mycharacter (Variables|Default|GetMyCharacter))
  ;[1 1 1] Input Movement
  (Utilities|IsValid _mycharacter
    (:Is%20Valid
      (Class|MainCharacter|MoveForward _mycharacter AxisValue))))

(event Input|AxisEvents|InputAxisMoveRight
  (params (AxisValue :type Float%20%28single-precision%29))
  (bind _mycharacter (Variables|Default|GetMyCharacter))
  ;[1 1 1] Input Movement
  (Utilities|IsValid _mycharacter
    (:Is%20Valid
      (Class|MainCharacter|MoveRight _mycharacter AxisValue))))

(fn ConstructionScript)

(fn OnInventoryNavigate
  (params (Direction :type EDirectionType%20Enum :default "VE_NONE"))
  (bind _mycharacter (Variables|Default|GetMyCharacter))
  (Utilities|IsValid _mycharacter
    (:Is%20Valid
      (if (Class|MainCharacter|IsInventoryActive _mycharacter)
        (Class|LobbyPlayerController|ClientNavigateInventory Direction)
        (else
          (return))))))

(fn IsInventoryReady
  (bind _mycharacter (Variables|Default|GetMyCharacter))
  (if (Pawn|IsLocalController)
    (Utilities|IsValid _mycharacter
      (:Is%20Valid
        (if (Class|MainCharacter|IsInventoryActive _mycharacter)
          (return true _mycharacter)
          (else
            (return false _mycharacter)))))))