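; Interactive door for Room 1 that swings open when its use event fires.
; The DoorOpening timeline drives a lerp on the mesh's world yaw across a quarter turn, keeping roll and pitch unchanged.
; The same event also starts the door audio and makes a point light visible.
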(event EventOnUseEvent
  (bind _mesh (Variables|Character|GetMesh))
  (bind _returnvalue (Transformation|GetWorldRotation _mesh))
  (Utilities|FlowControl|Sequence
    (:then_0
      (bind _yawrotation (Timeline|DoorOpening Play)
        (:Update
          (Transformation|SetWorldRotation (Variables|Character|GetMesh) (Math|Rotator|MakeRotator (.roll _returnvalue) (.pitch _returnvalue) (Math|Float|Lerp 9e+01 0.0 _yawrotation)) false false))))
    (:then_1
      (Audio|Components|Audio|Play (Variables|Default|GetAudio) 0.0))
    (:then_2
      (Rendering|SetVisibility (Variables|Default|GetPointLight) true false))))

(fn ConstructionScript)