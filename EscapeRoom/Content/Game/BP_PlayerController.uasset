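; Player controller Blueprint that turns inventory input actions into inventory toggle and navigation calls.
; On BeginPlay it caches the controlled pawn as a MainCharacter reference.
; Left and right presses send a direction through ClientNavigateInventory and releases send NONE, while the toggle action calls ClientToggleInventory.
; OnInventoryNavigate forwards a direction to the same call when the cached character is valid, behind an always-true branch.
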(event EventBeginPlay
  ;[1 1 1] Set Character
  (bind _asmain_character (Utilities|Casting|CastToMainCharacter (Pawn|GetControlledPawn)))
  (Variables|Default|SetMyCharacter _asmain_character))

(event Input|ActionEvents|InputActionInputToggleInventory
  (params (Key :type Key%20Structure))
  ;[1 1 1] Inventory Navigation
  (:Pressed
    (Class|LobbyPlayerController|ClientToggleInventory)))

(event Input|ActionEvents|InputActionNavigateInventoryLeft
  (params (Key :type Key%20Structure))
  ;[1 1 1] Inventory Navigation
  (:Pressed
    (Class|LobbyPlayerController|ClientNavigateInventory "VE_LEFT"))
  (:Released
    (Class|LobbyPlayerController|ClientNavigateInventory "VE_NONE")))

(event Input|ActionEvents|InputActionNavigateInventoryRight
  (params (Key :type Key%20Structure))
  ;[1 1 1] Inventory Navigation
  (:Pressed
    (Class|LobbyPlayerController|ClientNavigateInventory "VE_RIGHT"))
  (:Released
    (Class|LobbyPlayerController|ClientNavigateInventory "VE_NONE")))

(fn ConstructionScript)

(fn OnInventoryNavigate
  (params (Direction :type EDirectionType%20Enum :default "VE_NONE"))
  (Utilities|IsValid (Variables|Default|GetMyCharacter)
    (:Is%20Valid
      (if true
        (Class|LobbyPlayerController|ClientNavigateInventory Direction)
        (else
          (return))))))