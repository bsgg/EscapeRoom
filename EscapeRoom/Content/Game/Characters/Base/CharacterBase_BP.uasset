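; Base character Blueprint that gives the player an in-game HUD and shows network role and inventory debug information.
; On BeginPlay it creates an InGamePlayer_WBP widget, without a local-control check, and labels it server or client by authority, removing it on EndPlay.
; Each Tick, the locally controlled character prints its InventoryComponent object count on screen.
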(event EventEndPlay
  (params (EndPlayReason :type EEndPlayReason%20Enum :default "Destroyed"))
  (Widget|RemovefromParent (stale EventBeginPlay _returnvalue)))

(event Collision|EventActorBeginOverlap
  (params (OtherActor :type Actor%20Object%20Reference)))

(event EventBeginPlay
  (bind _returnvalue (UserInterface|CreateWidget "/Game/Game/UI/InGamePlayer_WBP.InGamePlayer_WBP_C"))
  (UserInterface|Viewport|AddtoViewport _returnvalue 0)
  (Networking|SwitchHasAuthority
    (:Authority
      (Rendering|Components|TextRender|SetText (Variables|/Game/Game/UI/InGamePlayer_WBP.InGamePlayer_WBP_C|GetInGameMessages _returnvalue) "I am server"))
    (:Remote
      (Rendering|Components|TextRender|SetText (Variables|/Game/Game/UI/InGamePlayer_WBP.InGamePlayer_WBP_C|GetInGameMessages _returnvalue) "I am client"))))

(event EventTick
  (params (DeltaSeconds :type Float%20%28single-precision%29))
  (if (Pawn|IsLocallyControlled)
    (Development|PrintString (Utilities|String|Append "Number Of Objects in Inventory: " (Utilities|String|ToString(Integer) (Variables|/Script/EscapeRoom.InventoryComponent|GetObjectNum (Variables|Default|GetInventoryComponent)))) true false "(R=0.000000,G=0.660000,B=1.000000,A=1.000000)" 0.0)))

(fn ConstructionScript)